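; Game mode for Obstacle Assault that respawns the player's third-person character.
; RespawnPlayer prints a wait message, pauses for a second, then spawns a new character and has the first player controller possess it.
; The spawn uses the POS component transform of LastCheckpoint when valid, otherwise a hard-coded world location, and always spawns regardless of collision.
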(event `Respawn Player`
  (`KismetSystemLibrary.PrintString` "wait a second")
  (`KismetSystemLibrary.Delay` 1.0)
  (bind _last_checkpoint (`self.last checkpoint`)
    (:`then`
      (bind (_returnvalue_location _returnvalue_rotation) (`KismetMathLibrary.BreakTransform` (`SceneComponent.K2_GetComponentToWorld` (`/Game/BP_Checkpoint.POS` _last_checkpoint))))
      (bind _returnvalue (`|SpawnActorFromClass` "/Game/BP_ThirdPersonCharacter.BP_ThirdPersonCharacter_C" (`KismetMathLibrary.MakeTransform` _returnvalue_location _returnvalue_rotation) "AlwaysSpawn" "MultiplyWithRoot" null null))
      (`Controller.Possess` (`GameplayStatics.GetPlayerController` 0) _returnvalue))
    (:`else`
      (bind _returnvalue_2 (`|SpawnActorFromClass` "/Game/BP_ThirdPersonCharacter.BP_ThirdPersonCharacter_C" (`KismetMathLibrary.MakeTransform` (-13990.0 -8670.0 4052.0)) "AlwaysSpawn" "MultiplyWithRoot" null null))
      (`Controller.Possess` (`GameplayStatics.GetPlayerController` 0) _returnvalue_2))))

(fn `UserConstructionScript`)